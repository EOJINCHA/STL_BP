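; BP_SandBag is a damageable AI actor that moves toward pawns it sees and is destroyed when its health runs out.
; PawnSensing's OnSeePawn issues an AIMoveTo on itself, targeting whichever pawn was seen.
; AnyDamage feeds SetHelath, which clamps Health between zero and its current value, so it cannot rise, and sets IsDead at zero, triggering DestroyActor.
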(event OnSeePawn(PawnSensing)
  (params (Pawn :type Pawn%20Object%20Reference))
  (AI|AIMoveTo self "0, 0, 0" Pawn 5.0 false))

(event EventBeginPlay)

(event Collision|EventActorBeginOverlap
  (params (OtherActor :type Actor%20Object%20Reference)))

(event EventTick
  (params (DeltaSeconds :type Float%20%28single-precision%29)))

(event Game|Damage|EventAnyDamage
  (params (Damage :type Float%20%28single-precision%29) (DamageType :type Damage%20Type%20Object%20Reference) (InstigatedBy :type Controller%20Object%20Reference) (DamageCauser :type Actor%20Object%20Reference))
  (CallFunction|SetHelath Damage)
  (if (Variables|Default|GetbIsDead)
    (Actor|DestroyActor)))

(fn ConstructionScript)

(fn SetHelath
  (params (Damage :type Float%20%28double-precision%29))
  (bind _output_get (Variables|Default|SetHealth (Math|Float|Clamp(Float) (- (Variables|Default|GetHealth) Damage) 0.0 (Variables|Default|GetHealth))))
  (if (== _output_get 0.0)
    (Variables|Default|SetbIsDead true)))