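; Swinging gate actor that opens away from the player's pawn when it enters the trigger box.
; CheckDir uses a dot product of gate forward and pawn-to-gate direction to set swing sign, also printing it.
; Open and close timelines lerp SMDoor's yaw from its current angle, each stopping the other.
; The gate closes on the player's exit or a timer after fully opening; OpenGate and CloseGate are unused here.
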(event OnComponentBeginOverlap(Box)
  (params (OverlappedComponent :type Primitive%20Component%20Object%20Reference) (OtherActor :type Actor%20Object%20Reference) (OtherComp :type Primitive%20Component%20Object%20Reference) (OtherBodyIndex :type Integer) (bFromSweep :type Boolean) (SweepResult :type Hit%20Result%20Structure%20%28by%20ref%29))
  ;[1 1 1] 트리거 조건 예외처리(내캐릭터인 경우만)
  (if (== OtherActor (Pawn|GetControlledPawn (Game|GetPlayerController 0)))
    (CallFunction|DoorCloseStop)
    (CallFunction|CheckDir)
    (Variables|Default|SetCurrentYaw (.yaw (Variables|/Script/Engine.SceneComponent|GetRelativeRotation (Variables|Default|GetSM_Door))))
    (Variables|Default|SetTargetYaw 9e+01)
    (bind _alpha (Timeline|TL_DoorOpen PlayFromStart)
      (:Update
        (CallFunction|OpenDynamicGate _alpha))
      (:Finished
        (Utilities|Time|SetTimerbyEvent (delegate Custom|CloseDoorByTimer) 3.0)))))

(event OnComponentEndOverlap(Box)
  (params (OverlappedComponent :type Primitive%20Component%20Object%20Reference) (OtherActor :type Actor%20Object%20Reference) (OtherComp :type Primitive%20Component%20Object%20Reference) (OtherBodyIndex :type Integer))
  (bind _returnvalue (Game|GetPlayerController 0))
  (Utilities|IsValid _returnvalue
    (:Is%20Valid
      (if (== OtherActor (Pawn|GetControlledPawn _returnvalue))
        (CallFunction|DoorOpenStop)
        (Variables|Default|SetCurrentYaw (.yaw (Variables|/Script/Engine.SceneComponent|GetRelativeRotation (Variables|Default|GetSM_Door))))
        (Variables|Default|SetTargetYaw 0.0)
        (bind _새_트랙_0 (Timeline|TL_DoorClose PlayFromStart)
          (:Update
            (CallFunction|CloseDynamicGate _새_트랙_0)))))))

(event Custom|DoorOpen_Stop
  (bind _alpha (Timeline|TL_DoorOpen Stop)
    (:Update
      (CallFunction|OpenDynamicGate _alpha))
    (:Finished
      (Utilities|Time|SetTimerbyEvent (delegate Custom|CloseDoorByTimer) 3.0))))

(event Custom|DoorClose_Stop
  (bind _새_트랙_0 (Timeline|TL_DoorClose Stop)
    (:Update
      (CallFunction|CloseDynamicGate _새_트랙_0))))

(event Custom|CloseDoorByTimer
  (CallFunction|DoorOpenStop)
  (Variables|Default|SetCurrentYaw (.yaw (Variables|/Script/Engine.SceneComponent|GetRelativeRotation (Variables|Default|GetSM_Door))))
  (Variables|Default|SetTargetYaw 0.0)
  (bind _새_트랙_0 (Timeline|TL_DoorClose PlayFromStart)
    (:Update
      (CallFunction|CloseDynamicGate _새_트랙_0))))

(event EventBeginPlay)

(fn ConstructionScript)

(fn OpenGate
  (params (bIsBegin :type Boolean))
  (if bIsBegin
    (if (> (Math|Vector|DotProduct (Transformation|GetActorForwardVector) (Math|Vector|Normalize (- (Transformation|GetActorLocation) (Transformation|GetActorLocation (Pawn|GetControlledPawn (Game|GetPlayerController 0)))))) 0.0)
      (Transformation|SetRelativeRotation (Variables|Default|GetSM_Door) "0,180.000000, 0" false false)
      (else
        (Transformation|SetRelativeRotation (Variables|Default|GetSM_Door) "0, 0, 0" false false)))
    (else
      (Transformation|SetRelativeRotation (Variables|Default|GetSM_Door) "0,90.000000, 0" false false))))

(fn CloseGate)

(fn OpenDynamicGate
  (params (Alpha :type Float%20%28double-precision%29))
  (Transformation|SetRelativeRotation (Variables|Default|GetSM_Door) (Math|Rotator|MakeRotator 0.0 0.0 (Math|Float|Lerp (Variables|Default|GetCurrentYaw) (* (Variables|Default|GetDir) (Variables|Default|GetTargetYaw)) Alpha)) false false))

(fn CheckDir
  (bind _returnvalue (Transformation|GetActorForwardVector))
  (bind _returnvalue_2 (Transformation|GetActorLocation))
  (bind _returnvalue_3 (Game|GetPlayerController 0))
  (bind _returnvalue_4 (Pawn|GetControlledPawn _returnvalue_3))
  (bind _returnvalue_5 (Transformation|GetActorLocation _returnvalue_4))
  (bind _returnvalue_6 (- _returnvalue_2 _returnvalue_5))
  (bind _returnvalue_7 (Math|Vector|Normalize _returnvalue_6))
  (bind _returnvalue_8 (Math|Vector|DotProduct _returnvalue_7 _returnvalue))
  (Development|PrintString (Utilities|String|ToString(Float) _returnvalue_8))
  (if (> _returnvalue_8 0.0)
    (Variables|Default|SetDir 1.0)
    (else
      (Variables|Default|SetDir -1.0))))

(fn CloseDynamicGate
  (params (Alpha :type Float%20%28double-precision%29))
  (Transformation|SetRelativeRotation (Variables|Default|GetSM_Door) (Math|Rotator|MakeRotator 0.0 0.0 (Math|Float|Lerp (Variables|Default|GetTargetYaw) (Variables|Default|GetCurrentYaw) Alpha)) false false))