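; BP_ItemBox is a weapon pickup box that gives a weapon to a character touching it.
; On overlap with a BP_Character, it checks CanGetWeapon, then spawns its Weapon class owned by that character and adds it to a slot, or prints "Full Slot".
; The construction script assigns the box a random mesh from its Meshes array.
; The box is not destroyed or disabled after a pickup.
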(event OnComponentBeginOverlap(ItemBox)
  (params (OverlappedComponent :type Primitive%20Component%20Object%20Reference) (OtherActor :type Actor%20Object%20Reference) (OtherComp :type Primitive%20Component%20Object%20Reference) (OtherBodyIndex :type Integer) (bFromSweep :type Boolean) (SweepResult :type Hit%20Result%20Structure%20%28by%20ref%29))
  (bind _asbp_character (Utilities|Casting|CastToBP_Character OtherActor))
  (bind _bcangetweapon (Default|CanGetWeapon _asbp_character))
  (if _bcangetweapon
    (bind _returnvalue (Game|SpawnActorfromClass (Variables|Default|GetWeapon) (Math|Transform|MakeTransform "0, 0, 0") "AlwaysSpawn" _asbp_character 0))
    (Default|AddWeapontoSlot _asbp_character _returnvalue)
    (else
      (Development|PrintString "Full Slot"))))

(fn ConstructionScript
  (Components|StaticMesh|SetStaticMesh (Variables|Default|GetItemBox) (.OutItem (Utilities|Array|Random (Variables|Default|GetMeshes)))))