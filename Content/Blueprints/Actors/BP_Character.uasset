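; Player character with movement, interface-based interaction, two-slot weapon swapping, combo melee attacks, damage, timed respawn and leveling.
; Attack input queues combos through AnimInstance callbacks that jump montage sections, with a separate section while falling.
; Tick sphere-traces between trail sockets to apply damage while IsAttackCheck is set.
; Level stats come from BP_Gameinstance, whose LoadData also restores HP, weapons and location on BeginPlay.
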(event OnComponentBeginOverlap(InteractCollision)
  (params (OverlappedComponent :type Primitive%20Component%20Object%20Reference) (OtherActor :type Actor%20Object%20Reference) (OtherComp :type Primitive%20Component%20Object%20Reference) (OtherBodyIndex :type Integer) (bFromSweep :type Boolean) (SweepResult :type Hit%20Result%20Structure%20%28by%20ref%29))
  ;[1 1 1] BPI있는 액터인 경우 레퍼런스 등록
  (if (Utilities|DoesObjectImplementInterface OtherActor "/Game/Blueprints/Interface/BPI_Interact.BPI_Interact_C")
    (Variables|Default|SetInteractTarget OtherActor)))

(event OnComponentEndOverlap(InteractCollision)
  (params (OverlappedComponent :type Primitive%20Component%20Object%20Reference) (OtherActor :type Actor%20Object%20Reference) (OtherComp :type Primitive%20Component%20Object%20Reference) (OtherBodyIndex :type Integer))
  ;[1 1 1] 감지 해제 시 레퍼 날려준다
  (if (== OtherActor (Variables|Default|GetInteractTarget))
    (Variables|Default|SetInteractTarget 0)))

(event Custom|OnNextAttackCheck
  (if (Variables|Attack|GetbIsComboInputOn)
    (Attack|AttackStartCombo)
    (Default|JumptoAttackMontageSection (Variables|Default|GetAnimInstance) (Variables|Attack|GetCurrentCombo))
    (else
      (Animation|Montage|MontageStop (Variables|Default|GetAnimInstance) 0.25 0))))

(event Custom|OnAttackMontageEnded
  (Attack|AttackEndCombo))

(event EventBeginPlay
  (bind _asbp_gameinstance (Utilities|Casting|CastToBP_Gameinstance (Game|GetGameInstance)))
  (Utilities|IsValid (Variables|/Game/Blueprints/Actors/BP_Gameinstance.BP_Gameinstance_C|GetLoadData _asbp_gameinstance)
    (:Is%20Valid
      (CallFunction|LoadCharacterData))
    (:Is%20Not%20Valid
      _))
  (Input|DisableInput (Game|GetPlayerController 0))
  (bind _asabp_character (Utilities|Casting|CastToABP_Character (Components|SkeletalMesh|GetAnimInstance (Variables|Character|GetMesh))))
  (bind _output_get (Variables|Default|SetAnimInstance _asabp_character))
  (EventDispatchers|AssignOnNextAttackCheck _output_get (delegate Custom|OnNextAttackCheck))
  (EventDispatchers|AssignOnAttackMontageEnded _output_get (delegate Custom|OnAttackMontageEnded))
  (bind _returnvalue (UserInterface|CreateWidget "/Game/UI/UMG_PlayerHUD.UMG_PlayerHUD_C" (Game|GetPlayerController 0)))
  (UserInterface|Viewport|AddtoViewport _returnvalue 0)
  (Utilities|FlowControl|Delay 2.5)
  (Input|EnableInput (Game|GetPlayerController 0)))

(event Game|Damage|EventAnyDamage
  (params (Damage :type Float%20%28single-precision%29) (DamageType :type Damage%20Type%20Object%20Reference) (InstigatedBy :type Controller%20Object%20Reference) (DamageCauser :type Actor%20Object%20Reference))
  (Development|PrintString (Utilities|String|ToString(Float) Damage))
  (Development|PrintString (Utilities|GetDisplayName InstigatedBy))
  (Development|PrintString (Utilities|GetDisplayName DamageCauser))
  (CallFunction|SetHP Damage)
  (if (Variables|Default|GetbIsDead)
    (Utilities|FlowControl|DoOnce false :!label _label
      (:Completed
        (Utilities|FlowControl|Delay 5.0)
        (CallFunction|Respawn)
        (goto _label Reset)))))

(event EventTick
  (params (DeltaSeconds :type Float%20%28single-precision%29))
  (Attack|AttackCheck))

(event Input|ActionEvents|InputActionJump
  (params (Key :type Key%20Structure))
  ;[1 1 1] 점프
  (:Pressed
    (Character|Jump))
  (:Released
    (Character|StopJumping)))

(event Input|ActionEvents|InputActionInteract
  (params (Key :type Key%20Structure))
  ;[1 1 1] 인터랙션 / Ref Valid인 경우 메시지 전달
  (:Pressed
    (Utilities|IsValid (Variables|Default|GetInteractTarget)
      (:Is%20Valid
        (Class|BPIInteract|Interaction(Message) (Variables|Default|GetInteractTarget))))))

(event Input|ActionEvents|InputActionAttack
  (params (Key :type Key%20Structure))
  ;[1 1 1] 무기 세팅, 공격
  (:Pressed
    (Utilities|IsValid (Variables|Weapon|GetCurrentWeapon)
      (:Is%20Valid
        (Attack|Attack)))))

(event Input|ActionEvents|InputActionSwapWeapon1
  (params (Key :type Key%20Structure))
  ;[1 1 1] 무기 세팅, 공격
  (:Pressed
    (CallFunction|SwapWeapon1)))

(event Input|ActionEvents|InputActionSwapWeapon2
  (params (Key :type Key%20Structure))
  ;[1 1 1] 무기 세팅, 공격
  (:Pressed
    (CallFunction|SwapWeapon2)))

(event Input|AxisEvents|InputAxisMoveForward/MoveBackward
  (params (AxisValue :type Float%20%28single-precision%29))
  ;[1 1 1] 이동
  (Pawn|Input|AddMovementInput (Math|Vector|GetForwardVector (Math|Rotator|MakeRotator 0.0 0.0 (.yaw (Pawn|GetControlRotation :!class /Script/Engine.Pawn)))) AxisValue false))

(event Input|AxisEvents|InputAxisMoveRight/MoveLeft
  (params (AxisValue :type Float%20%28single-precision%29))
  ;[1 1 1] 이동
  (Pawn|Input|AddMovementInput (Math|Vector|GetRightVector (Math|Rotator|MakeRotator 0.0 0.0 (.yaw (Pawn|GetControlRotation :!class /Script/Engine.Pawn)))) AxisValue false))

(event Input|AxisEvents|InputAxisTurnRight/Left
  (params (AxisValue :type Float%20%28single-precision%29))
  ;[1 1 1] 회전
  (Pawn|Input|AddControllerYawInput AxisValue))

(event Input|AxisEvents|InputAxisLookUp/Down
  (params (AxisValue :type Float%20%28single-precision%29))
  ;[1 1 1] 회전
  (Pawn|Input|AddControllerPitchInput AxisValue))

(fn ConstructionScript
  (Class|SkinnedMeshComponent|SetSkeletalMesh (Variables|Character|GetMesh) (Utilities|Array|Get(acopy) (Variables|Default|GetSK_Mesh_Arr) (Math|Random|RandomInteger 17)) false)
  (bind _asbp_gameinstance (Utilities|Casting|CastToBP_Gameinstance (Game|GetGameInstance)))
  (bind _characterdata (Default|GetCharacterData _asbp_gameinstance (.level (Variables|Default|GetCurrentCharacterData))))
  (bind _output_get (Variables|Default|SetCurrentCharacterData _characterdata))
  (Variables|Default|SetCurrentHP (.MaxHP (Utilities|Struct|BreakF_CharacterData _output_get))))

(fn Attack
  (if (Variables|Attack|GetbIsAttacking)
    ;[1 1 1] 콤보 입력 감지
    (Variables|Attack|SetbIsComboInputOn true)
    (return)
    (else
      (Attack|AttackStartCombo)
      (Default|PlayAttackMontage (Variables|Default|GetAnimInstance))
      (Default|JumptoAttackMontageSection (Variables|Default|GetAnimInstance) (Variables|Attack|GetCurrentCombo))
      (Variables|Attack|SetbIsAttacking true))))

(fn AttackStartCombo
  (if (AI|Components|NavMovement|IsFalling (Variables|Character|GetCharacterMovement))
    (Variables|Attack|SetbCanNextCombo false)
    (Variables|Attack|SetbIsComboInputOn false)
    (Variables|Attack|SetCurrentCombo 4)
    (else
      (Variables|Attack|SetbCanNextCombo true)
      (Variables|Attack|SetbIsComboInputOn false)
      (Variables|Attack|SetCurrentCombo (Math|Integer|Clamp(Integer) (+ (Variables|Attack|GetCurrentCombo) 1) 1 (Variables|Attack|GetMaxCombo))))))

(fn AttackEndCombo
  (Variables|Attack|SetbCanNextCombo false)
  (Variables|Attack|SetbIsComboInputOn false)
  (Variables|Attack|SetCurrentCombo 0)
  (Variables|Attack|SetbIsAttacking false)
  (Variables|/Script/Engine.CharacterMovementComponent|SetMaxWalkSpeed (Variables|Character|GetCharacterMovement) 6e+02))

(fn AttackCheck
  (bind _self self)
  (bind _mesh (Variables|Character|GetMesh))
  (if (Variables|Default|GetbIsAttackCheck)
    (bind _outhit (Collision|SphereTraceByChannel (Transformation|GetSocketLocation _mesh "Trail_Start") (Transformation|GetSocketLocation _mesh "Trail_End") 15.0 "TraceTypeQuery3" false (Variables|Default|GetHittedActor) "ForDuration" true "(R=1.000000,G=0.000000,B=0.000000,A=1.000000)" "(R=0.000000,G=1.000000,B=0.000000,A=1.000000)" 2.0))
    (Game|Damage|ApplyDamage (.hitactor _outhit) (.attack (Variables|Default|GetCurrentCharacterData)) (Pawn|GetController _self) _self)
    (Utilities|Array|AddUnique (Variables|Default|GetHittedActor) (.hitactor _outhit))
    (else
      (return))))

(fn CanGetWeapon
  (return (not (and (Utilities|IsValid (Variables|Weapon|GetWeaponSlot2)) (Utilities|IsValid (Variables|Weapon|GetWeaponSlot1))))))

(fn SetCurrentWeapon
  (params (NewWeapon :type BP%20Weapon%20Object%20Reference)))

(fn AddWeapontoSlot
  (params (NewWeapon :type BP%20Weapon%20Object%20Reference))
  (if (Utilities|IsValid (Variables|Weapon|GetWeaponSlot1))
    (if (not (Utilities|IsValid (Variables|Weapon|GetWeaponSlot2)))
      (bind _output_get (Variables|Weapon|SetWeaponSlot2 NewWeapon))
      (Transformation|AttachComponentToComponent _output_get (Variables|Character|GetMesh) "WeaponSlot2" "SnapToTarget" "SnapToTarget" "SnapToTarget" true))
    (else
      (bind _output_get_2 (Variables|Weapon|SetWeaponSlot1 NewWeapon))
      (Transformation|AttachComponentToComponent (Variables|Weapon|GetWeaponSlot1) (Variables|Character|GetMesh) "WeaponSlot1" "SnapToTarget" "SnapToTarget" "SnapToTarget" true))))

(fn SwapWeapon1
  (Utilities|IsValid (Variables|Weapon|GetCurrentWeapon)
    (:Is%20Valid
      ;[1 1 1] 장착한 무기가 있음
      (Utilities|IsValid (Variables|Weapon|GetWeaponSlot1)
        (:Is%20Valid
          ;[1 1 1] 현재 무기가 있는데/ 1번 슬롯과 비교
          (if (== (Variables|Weapon|GetWeaponSlot1) (Variables|Weapon|GetCurrentWeapon))
            ;[1 1 1] 현재 무기가 1번 슬롯 무기여서 뺀다 = 등에 붙임
            (Variables|Weapon|SetCurrentWeapon 0)
            (Transformation|AttachComponentToComponent (Variables|Weapon|GetWeaponSlot1) (Variables|Character|GetMesh) "WeaponSlot1" "SnapToTarget" "SnapToTarget" "SnapToTarget" true)
            (else
              ;[1 1 1] 현재 무기가 1번이 아님/ == 2번 무기 사용중 -> 2번 무기 등으로 보내고, 1번 무기 착용
              (Transformation|AttachComponentToComponent (Variables|Weapon|GetWeaponSlot2) (Variables|Character|GetMesh) "WeaponSlot2" "SnapToTarget" "SnapToTarget" "SnapToTarget" true)
              (bind _output_get (Variables|Weapon|SetCurrentWeapon (Variables|Weapon|GetWeaponSlot1)))
              (Transformation|AttachComponentToComponent _output_get (Variables|Character|GetMesh) "R_Weapon" "SnapToTarget" "SnapToTarget" "SnapToTarget" true))))))
    (:Is%20Not%20Valid
      ;[1 1 1] 맨손인데 무기슬롯1번에 무기가 있어서/ 1번 무기 바로 장착
      (Utilities|IsValid (Variables|Weapon|GetWeaponSlot1)
        (:Is%20Valid
          (bind _output_get_2 (Variables|Weapon|SetCurrentWeapon (Variables|Weapon|GetWeaponSlot1)))
          (Transformation|AttachComponentToComponent _output_get_2 (Variables|Character|GetMesh) "R_Weapon" "SnapToTarget" "SnapToTarget" "SnapToTarget" true))))))

(fn SwapWeapon2
  (if (Utilities|IsValid (Variables|Weapon|GetWeaponSlot2))
    (if (== (Variables|Weapon|GetCurrentWeapon) (Variables|Weapon|GetWeaponSlot2))
      (Variables|Weapon|SetCurrentWeapon 0)
      (Transformation|AttachComponentToComponent (Variables|Weapon|GetWeaponSlot2) (Variables|Character|GetMesh) "WeaponSlot2" "SnapToTarget" "SnapToTarget" "SnapToTarget" true)
      (else
        (Variables|Weapon|SetCurrentWeapon (Variables|Weapon|GetWeaponSlot2))
        (Transformation|AttachComponentToComponent (Variables|Weapon|GetWeaponSlot1) (Variables|Character|GetMesh) "WeaponSlot1" "SnapToTarget" "SnapToTarget" "SnapToTarget" true)
        (Transformation|AttachComponentToComponent (Variables|Weapon|GetWeaponSlot2) (Variables|Character|GetMesh) "R_Weapon" "SnapToTarget" "SnapToTarget" "SnapToTarget" true)))))

(fn SetHP
  (params (Damage :type Float%20%28double-precision%29))
  (bind _output_get (Variables|Default|SetCurrentHP (- (Variables|Default|GetCurrentHP) Damage)))
  (Development|PrintString (Utilities|String|Append "CurrentHP:" (Utilities|String|ToString(Float) _output_get)))
  (if (<= (Variables|Default|GetCurrentHP) 0.0)
    (Variables|Default|SetbIsDead true)
    (Input|DisableInput (Game|Player|GetPlayerPawn 0) (Game|GetPlayerController 0))
    (else
      (Variables|Default|SetbIsDead false))))

(fn Respawn
  (Variables|Default|SetCurrentHP (.MaxHP (Utilities|Struct|BreakF_CharacterData (Variables|Default|GetCurrentCharacterData))))
  (Variables|Default|SetbIsDead false)
  (Input|EnableInput (Game|Player|GetPlayerPawn 0) (Game|GetPlayerController 0)))

(fn GetExp
  (params (NewExp :type Float%20%28double-precision%29))
  (bind _output_get (Variables|Default|SetCurrentExp (+ NewExp (Variables|Default|GetCurrentExp))))
  (if (>= _output_get (.NextExp (Utilities|Struct|BreakF_CharacterData (Variables|Default|GetCurrentCharacterData))))
    (레벨|LevelUp)))

(fn LevelUp
  (bind _structout (Utilities|Struct|SetmembersinF_CharacterData (Variables|Default|GetCurrentCharacterData) (+ (.Level (Utilities|Struct|BreakF_CharacterData (Variables|Default|GetCurrentCharacterData))) 1)))
  (bind _asbp_gameinstance (Utilities|Casting|CastToBP_Gameinstance (Game|GetGameInstance)))
  (bind _characterdata (Default|GetCharacterData _asbp_gameinstance (.Level (Utilities|Struct|BreakF_CharacterData _structout))))
  ;[1 1 1] 레벨업 캐릭터의 데이터 신규 세팅
  (bind _output_get (Variables|Default|SetCurrentCharacterData _characterdata))
  (Variables|Default|SetCurrentHP (.MaxHP (Utilities|Struct|BreakF_CharacterData _output_get)))
  (Variables|Default|SetCurrentExp 0.0))

(fn GetExpRatio
  (return (/ (Variables|Default|GetCurrentExp) (.NextExp (Utilities|Struct|BreakF_CharacterData (Variables|Default|GetCurrentCharacterData))))))

(fn LoadCharacterData
  (bind _returnvalue (Math|Transform|MakeTransform "0, 0, 0"))
  (bind _asbp_gameinstance (Utilities|Casting|CastToBP_Gameinstance (Game|GetGameInstance)))
  (bind _characterdata (Default|GetCharacterData _asbp_gameinstance (Variables|/Game/Blueprints/BP_Savegame.BP_Savegame_C|GetCharacterLevel (Variables|/Game/Blueprints/Actors/BP_Gameinstance.BP_Gameinstance_C|GetLoadData _asbp_gameinstance))))
  (Variables|Default|SetCurrentCharacterData _characterdata)
  (Variables|Default|SetCurrentHP (Variables|/Game/Blueprints/BP_Savegame.BP_Savegame_C|GetCurrentHP (Variables|/Game/Blueprints/Actors/BP_Gameinstance.BP_Gameinstance_C|GetLoadData _asbp_gameinstance)))
  (bind _returnvalue_2 (Game|SpawnActorfromClass (Variables|/Game/Blueprints/BP_Savegame.BP_Savegame_C|GetWeapon1 (Variables|/Game/Blueprints/Actors/BP_Gameinstance.BP_Gameinstance_C|GetLoadData _asbp_gameinstance)) _returnvalue "AlwaysSpawn" 0 0))
  (CallFunction|AddWeapontoSlot _returnvalue_2)
  (bind _returnvalue_3 (Game|SpawnActorfromClass (Variables|/Game/Blueprints/BP_Savegame.BP_Savegame_C|GetWeapon2 (Variables|/Game/Blueprints/Actors/BP_Gameinstance.BP_Gameinstance_C|GetLoadData _asbp_gameinstance)) _returnvalue "AlwaysSpawn" 0 0))
  (CallFunction|AddWeapontoSlot _returnvalue_3)
  (Transformation|SetActorLocation (Variables|/Game/Blueprints/BP_Savegame.BP_Savegame_C|GetActorLocation (Variables|/Game/Blueprints/Actors/BP_Gameinstance.BP_Gameinstance_C|GetLoadData _asbp_gameinstance)) false false)
  (Variables|/Game/Blueprints/Actors/BP_Gameinstance.BP_Gameinstance_C|SetLoadData _asbp_gameinstance 0))