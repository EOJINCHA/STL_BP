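; Bear enemy character with data table stats, a health bar widget and a blackboard state that also sets walk speed.
; Pawn sensing sets the first player seen as chase target.
; The attack collision collects overlapped actors while enabled, then damages them all when disabled.
; Damage triggers a hit flash; death stops AI logic, dissolves the mesh, grants EXP to the damage causer, notifies its spawner and destroys the bear.
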(event OnSeePawn(PawnSensing)
  (params (Pawn :type Pawn%20Object%20Reference))
  (bind _asbp_character (Utilities|Casting|CastToBP_Character Pawn))
  (Utilities|FlowControl|DoOnce false
    (:Completed
      (AI|Components|Blackboard|SetValueasObject (AI|GetBlackboard (Pawn|GetController)) (Utilities|Name|MakeLiteralName "TargetPlayer") _asbp_character)
      (CallFunction|SetState "NewEnumerator1"))))

(event OnComponentBeginOverlap(AttackCollision)
  (params (OverlappedComponent :type Primitive%20Component%20Object%20Reference) (OtherActor :type Actor%20Object%20Reference) (OtherComp :type Primitive%20Component%20Object%20Reference) (OtherBodyIndex :type Integer) (bFromSweep :type Boolean) (SweepResult :type Hit%20Result%20Structure%20%28by%20ref%29))
  (Utilities|Array|AddUnique (Variables|Default|GetHittedActor) OtherActor))

(event Custom|HittedEffect
  (bind _color (Timeline|TL_HiitedEffect PlayFromStart)
    (:Update
      (Rendering|Material|SetVectorParameterValueonMaterials (Variables|Character|GetMesh) "HittedColor" (Math|Vector|MakeVector _color 0.0 0.0)))))

(event Custom|DissolveEffect
  (bind _parentspawner (Variables|Default|GetParentSpawner))
  (bind _damage_causer (Variables|Default|GetDamage%20Causer))
  (bind _새_트랙_0 (Timeline|타임라인_0 PlayFromStart)
    (:Update
      (Rendering|Material|SetScalarParameterValueonMaterials (Variables|Character|GetMesh) "DissolveIntensity" _새_트랙_0))
    (:Finished
      (Utilities|IsValid _damage_causer
        (:Is%20Valid
          (bind _asbp_character (Utilities|Casting|CastToBP_Character _damage_causer)
            (:then
              (Default|GetExp _asbp_character (.DropExp (Utilities|Struct|BreakF_BearData (Variables|Default|GetCurrentStat)))))
            (:CastFailed
              _)))
        (:Is%20Not%20Valid
          _))
      (Utilities|IsValid _parentspawner
        (:Is%20Valid
          (Default|RemoveDeadBear _parentspawner self))
        (:Is%20Not%20Valid
          _))
      (Actor|DestroyActor))))

(event EventBeginPlay
  (bind _wb_healthbar (Variables|Default|GetWB_Healthbar))
  (bind _returnvalue (UserInterface|GetWidget _wb_healthbar))
  (Development|PrintString (Utilities|GetDisplayName _returnvalue))
  (bind _asumg_enemy_healthbar (Utilities|Casting|CastToUMG_EnemyHealthbar _returnvalue))
  (Variables|/Game/UI/UMG_EnemyHealthbar.UMG_EnemyHealthbar_C|SetOwner _asumg_enemy_healthbar self))

(event Collision|EventActorBeginOverlap
  (params (OtherActor :type Actor%20Object%20Reference)))

(event EventTick
  (params (DeltaSeconds :type Float%20%28single-precision%29)))

(event Game|Damage|EventAnyDamage
  (params (Damage :type Float%20%28single-precision%29) (DamageType :type Damage%20Type%20Object%20Reference) (InstigatedBy :type Controller%20Object%20Reference) (DamageCauser :type Actor%20Object%20Reference))
  (CallFunction|SetHealth Damage)
  (CallFunction|HittedEffect)
  (Variables|Default|SetDamage%20Causer DamageCauser))

(fn ConstructionScript
  (Collision|SetCollisionEnabled (Variables|Default|GetAttackCollision) "NoCollision")
  (bind _returnvalue (Utilities|GetDataTableRow "/Game/Blueprints/Actors/Bear/DT_BearData.DT_BearData" "1")
    (:then
      (bind _output_get (Variables|Default|SetCurrentStat _returnvalue))
      (Variables|Default|SetCurrentHp (.maxhp _output_get)))))

(fn SetAttackCollision
  (params (bIsEnable :type Boolean))
  (if bIsEnable
    (Collision|SetCollisionEnabled (Variables|Default|GetAttackCollision) "QueryOnly")
    (else
      (Collision|SetCollisionEnabled (Variables|Default|GetAttackCollision) "NoCollision")
      (for _array_element (Variables|Default|GetHittedActor)
        (Game|Damage|ApplyDamage _array_element (Variables|Default|GetAttackDamage) (Pawn|GetController) self))
      (Utilities|Array|Clear (Variables|Default|GetHittedActor)))))

(fn SetState
  (params (NewState :type E_BearState%20Enum :default "NewEnumerator0"))
  (bind _charactermovement (Variables|Character|GetCharacterMovement))
  (bind _output_get (Variables|Default|SetState NewState))
  (AI|Components|Blackboard|SetValueasEnum (AI|GetBlackboard (Pawn|GetController)) (Utilities|Name|MakeLiteralName "BearState") _output_get)
  (switch Utilities|FlowControl|Switch|SwitchonE_BearState (Variables|Default|GetState)
    (:NewEnumerator0
      (Variables|/Script/Engine.CharacterMovementComponent|SetMaxWalkSpeed _charactermovement 2e+02))
    (:NewEnumerator1
      (Variables|/Script/Engine.CharacterMovementComponent|SetMaxWalkSpeed _charactermovement 4e+02))
    (:NewEnumerator2
      (Variables|/Script/Engine.CharacterMovementComponent|SetMaxWalkSpeed _charactermovement 0.0 :!label _label))
    (:NewEnumerator3
      (goto _label))))

(fn GetHealthRatio
  (return (/ (Variables|Default|GetCurrentHp) (.MaxHp (Utilities|Struct|BreakF_BearData (Variables|Default|GetCurrentStat))))))

(fn SetHealth
  (params (NewDamage :type Float%20%28double-precision%29))
  (bind _output_get (Variables|Default|SetCurrentHp (- (Variables|Default|GetCurrentHp) NewDamage)))
  (if (<= _output_get 0.0)
    (Variables|Default|SetState "NewEnumerator3")
    (AI|Logic|StopLogic (Variables|/Script/AIModule.AIController|GetBrainComponent (AI|GetAIController self)) "")
    (Collision|SetCollisionEnabled (Variables|Collision|GetCapsuleComponent) "NoCollision")
    (CallFunction|DissolveEffect)))