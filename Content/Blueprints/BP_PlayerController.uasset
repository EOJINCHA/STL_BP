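; BP_PlayerController is a player controller that sets up game-only input and opens an in-game menu.
; On BeginPlay it starts a camera fade from fully opaque over a short duration.
; The Menu input action lazily creates the UMG_Menu widget, caches it, and re-adds it to the viewport at a high Z-order when it is not already shown.
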(event EventBeginPlay
  (Input|SetInputModeGameOnly self)
  (CameraFades|StartCameraFade :self (Variables|Default|GetPlayerCameraManager) :FromAlpha 1.0 :Duration 2.5))

(event Input|ActionEvents|InputActionMenu
  (params (Key :type Key%20Structure :default "None"))
  (:Pressed
    (Utilities|IsValid (Variables|Default|GetWB_Menu)
      (:Is%20Valid
        (if (not (UserInterface|Viewport|IsinViewport (Variables|Default|GetWB_Menu)))
          (UserInterface|Viewport|AddtoViewport (Variables|Default|GetWB_Menu) 99)))
      (:Is%20Not%20Valid
        (bind _returnvalue (UserInterface|CreateWidget "/Game/UI/UMG_Menu.UMG_Menu_C" (Game|GetPlayerController 0)))
        (bind _output_get (Variables|Default|SetWB_Menu _returnvalue))
        (UserInterface|Viewport|AddtoViewport _output_get 99)))))

(fn ConstructionScript)