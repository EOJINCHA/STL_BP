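; BP_MinimapCapturer is an actor that provides the minimap view through an orthographic SceneCaptureComponent2D.
; The construction script starts the capture's OrthoWidth at OrthoMin, the most zoomed-in level.
; ZoomIn and ZoomOut step OrthoWidth down or up by ZoomStep, clamped between OrthoMin and OrthoMax.
; The event graph holds no logic, so zooming happens only when those functions are called.
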(event EventBeginPlay)

(event Collision|EventActorBeginOverlap
  (params (OtherActor :type Actor%20Object%20Reference)))

(event EventTick
  (params (DeltaSeconds :type Float%20%28single-precision%29)))

(fn ConstructionScript
  (Variables|/Script/Engine.SceneCaptureComponent2D|SetOrthoWidth (Variables|Default|GetSceneCaptureComponent2D) (Variables|Default|GetOrthoMin)))

(fn Zoomin
  (bind _scenecapturecomponent2d (Variables|Default|GetSceneCaptureComponent2D))
  (Variables|/Script/Engine.SceneCaptureComponent2D|SetOrthoWidth _scenecapturecomponent2d (Math|Float|Clamp(Float) (- (Variables|/Script/Engine.SceneCaptureComponent2D|GetOrthoWidth _scenecapturecomponent2d) (Variables|Default|GetZoomStep)) (Variables|Default|GetOrthoMin) (Variables|Default|GetOrthoMax))))

(fn ZoomOut
  (bind _scenecapturecomponent2d (Variables|Default|GetSceneCaptureComponent2D))
  (Variables|/Script/Engine.SceneCaptureComponent2D|SetOrthoWidth _scenecapturecomponent2d (Math|Float|Clamp(Float) (+ (Variables|/Script/Engine.SceneCaptureComponent2D|GetOrthoWidth _scenecapturecomponent2d) (Variables|Default|GetZoomStep)) (Variables|Default|GetOrthoMin) (Variables|Default|GetOrthoMax))))